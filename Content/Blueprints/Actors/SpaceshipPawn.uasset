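; Player spaceship pawn that steers on the Y/Z plane, fires lasers and toggles exhaust particles.
; Axis input builds clamped speed and drift; drift tilts the mesh and eases toward zero on Tick unless CanFire is set.
; Tick also clamps position inside an invisible cage, while the deprecated forward movement is disconnected.
; PullTrigger and ReleaseTrigger, custom events because DefaultSpaceLevel consumes the input, start and stop timer-driven auto-fire.
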(event `self.ReceiveBeginPlay`)

(event `self.ReceiveActorBeginOverlap`
  (params (OtherActor :type "Actor Object Reference")))

(event `InputAxis|MoveUp`
  (params (AxisValue :type "Float (single-precision)"))
  ;[1 1 1] Move horizontal
  ;;[1 1 1] Hold maximum moving speed
  (bind _correctedvalue (`self.HoldMinMaxValue` (+ (`self.MovespeedRightLeft`) AxisValue) (`self.MAXPOSITIVEMOVESPEED`) (`self.MAXNEGATIVEMOVESPEED`)))
  (bind _output_get (set `self.MovespeedRightLeft` _correctedvalue))
  ;;[1 1 1] Add horizontal drift
  (bind _correctedvalue_2 (`self.HoldMinMaxValue` (+ AxisValue (`self.HorizontalDrift`)) (`self.MAXPOSITIVEDRIFT`) (`self.MAXNEGATIVEDRIFT`)))
  (set `self.HorizontalDrift` _correctedvalue_2)
  (`self.AddMovementInput` (0.0 0.03 0.0) _output_get))

(event `InputAxis|MoveRight`
  (params (AxisValue :type "Float (single-precision)"))
  ;[1 1 1] Move vertical
  ;;[1 1 1] Hold maximum moving speed
  (bind _correctedvalue (`self.HoldMinMaxValue` (+ (`self.MovespeedUpDown`) AxisValue) (`self.MAXPOSITIVEMOVESPEED`) (`self.MAXNEGATIVEMOVESPEED`)))
  (bind _output_get (set `self.MovespeedUpDown` _correctedvalue))
  ;;[1 1 1] Add vertical drift
  (bind _correctedvalue_2 (`self.HoldMinMaxValue` (+ AxisValue (`self.VerticalDrift`)) (`self.MAXPOSITIVEDRIFT`) (`self.MAXNEGATIVEDRIFT`)))
  (set `self.VerticalDrift` _correctedvalue_2)
  (`self.AddMovementInput` (0.0 0.0 0.03) _output_get))

(event `self.ReceiveTick`
  (params (DeltaSeconds :type "Float (single-precision)"))
  (bind _max_xy_coords_negative (`self.MAX_XY_COORDS_NEGATIVE`))
  (bind _max_xy_coords_positive (`self.MAX_XY_COORDS_POSITIVE`))
  (bind _verticaldrift (`self.VerticalDrift`))
  (bind _horizontaldrift (`self.HorizontalDrift`))
  (bind _defaultsceneroot (`self.DefaultSceneRoot`))
  (bind (_returnvalue_x _returnvalue_y _returnvalue_z) (`KismetMathLibrary.BreakVector` (`SceneComponent.K2_GetComponentLocation` _defaultsceneroot)))
  (bind _returnvalue (* DeltaSeconds (`self.ROTATIONRETURNSPEED`)))
  (bind _returnvalue_2 (* DeltaSeconds (`self.ROTATIONRETURNSPEED`)))
  ;[1 1 1] Move horizontal
  ;;[1 1 1] Continously drift correction for horizontal drift
  ;;;[1 1 1] Shootingpart, stop drift correction
  (if (`self.CanFire`)
    _
    (elif (< (`self.HorizontalDrift`) 0.0)
      (set `self.HorizontalDrift` (+ _horizontaldrift _returnvalue_2))
      (else
        (set `self.HorizontalDrift` (- _horizontaldrift _returnvalue_2)))))
  ;[1 1 1] Move vertical
  ;;[1 1 1] Continously drift correction for vertical drift
  ;;;[1 1 1] Shootingpart, stop drift correction
  (if (`self.CanFire`)
    _
    (elif (< (`self.VerticalDrift`) 0.0)
      (set `self.VerticalDrift` (+ _verticaldrift _returnvalue))
      (else
        (bind _output_get (set `self.VerticalDrift` (- _verticaldrift _returnvalue))))))
  ;[1 1 1] Paint actual rotation on screen
  (`SceneComponent.K2_SetRelativeRotation` (`self.SpaceshipMesh`) (`KismetMathLibrary.MakeRotator` _output_get 0.0 (+ 90.0 (`self.HorizontalDrift`))) false false)
  ;[1 1 1] Invisible cage for the ship
  (bind _correctedvalue (`self.HoldMinMaxValue` _returnvalue_y _max_xy_coords_positive _max_xy_coords_negative))
  (bind _correctedvalue_2 (`self.HoldMinMaxValue` _returnvalue_z _max_xy_coords_positive _max_xy_coords_negative))
  (`SceneComponent.K2_SetWorldLocation` _defaultsceneroot (`KismetMathLibrary.MakeVector` _returnvalue_x _correctedvalue _correctedvalue_2) false false))

(event `/Game/Blueprints/Interfaces/I_SpaceStationListener.SpacestationRingPassed`
  (params (Spacestation :type "/Game/Blueprints/Actors/SpacestationActor Object Reference") (RingID :type Integer) (Correctness :type "/Game/Blueprints/RingCorrectness Enum" :default "NewEnumerator0")))

(event `/Game/Blueprints/Interfaces/I_SpaceStationListener.SpacestationHitByPlayer`
  (params (StationHit :type "/Game/Blueprints/Actors/SpacestationActor Object Reference"))
  (`AudioComponent.Play` (`self.StationCollision`) 0.0))

(event `Fire`
  ;[1 1 1] Fire laser
  (`|SpawnActorFromClass` "/Game/Blueprints/Actors/BP_LaserProjectile.BP_LaserProjectile_C" (`SceneComponent.K2_GetComponentToWorld` (`self.ProjectileSpawningArrow`)) "Undefined" "OverrideRootScale"))

(event `PullTrigger`
  ;[1 1 1] Fire laser
  (if (`self.CanFire`)
    (`/Engine/EditorBlueprintResources/StandardMacros.DoOnce` false :!label _label
      (:`Completed`
        (`self.Fire`)
        (bind _returnvalue (`KismetSystemLibrary.K2_SetTimerDelegate` (delegate `Fire`) (/ 1.0 (`self.FireRate`)) true))))))

(event `ReleaseTrigger`
  ;[1 1 1] Fire laser
  (`KismetSystemLibrary.K2_ClearTimerHandle` (stale `PullTrigger` _returnvalue))
  (goto _label :!via `Reset`))

(fn `FireThrusters`
  (params (Active :type Boolean))
  (`ActorComponent.SetActive` (`self.ParticlesLeftExhaust`) Active false)
  (`ActorComponent.SetActive` (`self.ParticlesRightExhaust`) Active false))

(fn `HoldMinMaxValue`
  (params (inputValue :type "Float (double-precision)") (allowedMaximum :type "Float (double-precision)") (allowedMinimum :type "Float (double-precision)"))
  (returns (correctedValue :type "Float (double-precision)"))
  (return (`KismetMathLibrary.FMax` (`KismetMathLibrary.FMin` inputValue allowedMaximum) allowedMinimum)))

(fn `UserConstructionScript`)