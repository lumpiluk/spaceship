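; BP_Earth is an Earth actor with a surface sphere and an atmosphere whose shading follows a changeable light direction.
; The construction script creates dynamic materials for both meshes and sizes the atmosphere's eclipse parameter from its X scale.
; LightDirectionChanged feeds the negated direction to both materials and derives the atmosphere's eclipse position from it.
; ChangeRotationRate scales the RotatingMovement spin by a multiplier.
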(event `self.ReceiveBeginPlay`)

(event `self.ReceiveActorBeginOverlap`
  (params (OtherActor :type "Actor Object Reference")))

(event `self.ReceiveTick`
  (params (DeltaSeconds :type "Float (single-precision)")))

(event `/Game/Blueprints/Interfaces/I_LightDirectionObserver.LightDirectionChanged`
  (params (NewDirection :type "Vector Structure"))
  (`self.SetLightDirection` NewDirection))

(fn `ChangeRotationRate`
  (params (NewRateMultiplier :type "Float (double-precision)"))
  (set `RotatingMovementComponent.RotationRate` (`KismetMathLibrary.MakeRotator` 0.0 (* NewRateMultiplier 0.1) (* NewRateMultiplier 0.2)) (`self.RotatingMovement`)))

(fn `SetLightDirection`
  (params (NewDirection :type "Vector Structure"))
  (bind _returnvalue (`KismetMathLibrary.NegateVector` NewDirection))
  (bind _atmospherematerialdyn (`self.AtmosphereMaterialDyn`))
  (bind _returnvalue_2 (`KismetMathLibrary.Conv_VectorToLinearColor` _returnvalue))
  ;[1 1 1] Set light direction on earth
  (`MaterialInstanceDynamic.SetVectorParameterValue` (`self.EarthMaterialDyn`) "LightDirection" _returnvalue_2)
  ;[1 1 1] Set light direction on atmosphere
  (`MaterialInstanceDynamic.SetVectorParameterValue` _atmospherematerialdyn "LightDirection" _returnvalue_2)
  (`MaterialInstanceDynamic.SetVectorParameterValue` _atmospherematerialdyn "EclipsePositionA" (`KismetMathLibrary.Conv_VectorToLinearColor` (/ (+ (* (`KismetMathLibrary.Normal` _returnvalue) (`self.EclipsePositionDistanceFromEarthCenter`)) (`SceneComponent.K2_GetComponentLocation` (`self.Atmosphere`))) 2.0))))

(fn `UserConstructionScript`
  (bind _relativescale3d_x (`KismetMathLibrary.BreakVector` (`SceneComponent.RelativeScale3D` (`self.Atmosphere`))))
  (bind _returnvalue (`PrimitiveComponent.CreateDynamicMaterialInstance` (`self.Sphere`) 0 null))
  (set `self.EarthMaterialDyn` _returnvalue)
  (bind _returnvalue_2 (`PrimitiveComponent.CreateDynamicMaterialInstance` (`self.Atmosphere`) 0 null))
  (bind _output_get (set `self.AtmosphereMaterialDyn` _returnvalue_2))
  (`MaterialInstanceDynamic.SetScalarParameterValue` _output_get "EclipseSize" (* _relativescale3d_x 240.0)))