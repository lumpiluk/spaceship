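; BP_AsteroidFieldBounds is a moving volume marking an asteroid field that travels toward the player spaceship.
; Through I_Moveable it takes an oncoming speed as negative X projectile velocity and tells its moveable observer once it falls behind the player, allowing destruction.
; Two trigger volumes notify an asteroid observer when the tagged player enters shooting range or leaves the field bounds.
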(event `OnDestroyed_Event`)

(event `self.ReceiveBeginPlay`)

(event `self.ReceiveActorBeginOverlap`
  (params (OtherActor :type "Actor Object Reference")))

(event `self.ReceiveTick`
  (params (DeltaSeconds :type "Float (single-precision)"))
  (if (< (.x (.location (`self.GetTransform`))) (`self.BehindPlayerX`))
    ;[1 1 1] Notify observer that this actor can now be destroyed
    (`/Game/Blueprints/Interfaces/I_MoveableObserver.MoveableOutOfRange` (`self.MoveableObserver`) self)))

(event `self.AsteroidFieldShootingRange.OnComponentBeginOverlap`
  (params (OtherActor :type "Actor Object Reference") (OtherComp :type "PrimitiveComponent Object Reference") (OtherBodyIndex :type Integer) (bFromSweep :type Boolean) (SweepResult :type "HitResult Structure (by ref)"))
  (if (`self.ActorHasTag` OtherActor "SpaceshipPlayer")
    (if (`KismetSystemLibrary.IsValid` (`KismetSystemLibrary.Conv_InterfaceToObject` (`self.AsteroidObserver`)))
      (`/Game/Blueprints/Interfaces/I_AsteroidObserver.AsteroidFieldInShootingRange` (`self.AsteroidObserver`) self))))

(event `self.AsteroidFieldBounds.OnComponentEndOverlap`
  (params (OtherActor :type "Actor Object Reference") (OtherComp :type "PrimitiveComponent Object Reference") (OtherBodyIndex :type Integer))
  (if (`self.ActorHasTag` OtherActor "SpaceshipPlayer")
    (if (`KismetSystemLibrary.IsValid` (`KismetSystemLibrary.Conv_InterfaceToObject` (`self.AsteroidObserver`)))
      (`/Game/Blueprints/Interfaces/I_AsteroidObserver.AsteroidFieldBoundsLeft` (`self.AsteroidObserver`) self))))

(event `/Game/Blueprints/Interfaces/I_Moveable.SetOncomingSpeed`
  (params (NewSpeed :type "Float (single-precision)"))
  ;[1 1 1] I_Moveable implementations
  (set `MovementComponent.Velocity` (`KismetMathLibrary.MakeVector` (* NewSpeed -1.0)) (`self.ProjectileMovement`)))

(event `/Game/Blueprints/Interfaces/I_Moveable.SetObserver`
  (params (Observer :type "/Game/Blueprints/Interfaces/I_MoveableObserver Interface"))
  ;[1 1 1] I_Moveable implementations
  (set `self.MoveableObserver` Observer))

(event `/Game/Blueprints/Interfaces/I_Moveable.DestroyMoveableActor`
  ;[1 1 1] I_Moveable implementations
  (`self.K2_DestroyActor`))

(fn `UserConstructionScript`)