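; Billboard actor that shows three configurable text lines and moves toward -X at an externally set global speed via I_Moveable.
; Each Tick it reports to its Observer once behind the player's X threshold; otherwise it updates its ProjectileMovement velocity.
; With DoStop set, it lerps speed down by distance to StopAt, firing front thrusters until it drops below a small cutoff and halts.
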(event `self.ReceiveBeginPlay`)

(event `self.ReceiveActorBeginOverlap`
  (params (OtherActor :type "Actor Object Reference")))

(event `self.ReceiveTick`
  (params (DeltaSeconds :type "Float (single-precision)"))
  (bind _returnvalue (`KismetMathLibrary.Lerp` 0.0 (* (`self.GlobalSpeed`) -1.0) (`KismetMathLibrary.FClamp` (/ (- (.x (.location (`SceneComponent.K2_GetComponentToWorld` (`self.DefaultSceneRoot`)))) (`self.StopAt`)) (`KismetMathLibrary.Abs` (- (`self.StopBeginDecelerationAt`) (`self.StopAt`)))))))
  (if (< (.x (.location (`SceneComponent.K2_GetComponentToWorld` (`self.DefaultSceneRoot`)))) (`self.BehindPlayerX`))
    (`/Game/Blueprints/Interfaces/I_MoveableObserver.MoveableOutOfRange` (`self.Observer`) self)
    (else
      ;[1 1 1] Deceleration until StopAt
      (if (and (`self.DoStop`) (< (.x (.location (`SceneComponent.K2_GetComponentToWorld` (`self.DefaultSceneRoot`)))) (`self.StopBeginDecelerationAt`)))
        (set `MovementComponent.Velocity` (`KismetMathLibrary.MakeVector` _returnvalue) (`self.ProjectileMovement`))
        ;;[1 1 1] Set thrusters accordingly
        (if (< (`KismetMathLibrary.Abs` _returnvalue) 20.0)
          (`self.FireThrusters` false true)
          (set `MovementComponent.Velocity` (0.0 0.0 0.0) (`self.ProjectileMovement`))
          (else
            (`self.FireThrusters` true true)))
        (else
          (set `MovementComponent.Velocity` (`KismetMathLibrary.MakeVector` (* (`self.GlobalSpeed`) -1.0)) (`self.ProjectileMovement`)))))))

(event `/Game/Blueprints/Interfaces/I_Moveable.SetOncomingSpeed`
  (params (NewSpeed :type "Float (single-precision)"))
  ;[1 1 1] I_Moveable implementations
  (set `self.GlobalSpeed` NewSpeed))

(event `/Game/Blueprints/Interfaces/I_Moveable.SetObserver`
  (params (Observer :type "/Game/Blueprints/Interfaces/I_MoveableObserver Interface"))
  ;[1 1 1] I_Moveable implementations
  (set `self.Observer` Observer))

(event `/Game/Blueprints/Interfaces/I_Moveable.DestroyMoveableActor`
  ;[1 1 1] I_Moveable implementations
  (`self.K2_DestroyActor`))

(fn `FireThrusters`
  (params (Active :type Boolean) (AffectFront :type Boolean) (AffectBack :type Boolean))
  (if AffectFront
    (`ActorComponent.SetActive` (`self.Thruster00`) Active false)
    (`ActorComponent.SetActive` (`self.Thruster10`) Active false)
    (`ActorComponent.SetActive` (`self.Thruster20`) Active false)
    (`ActorComponent.SetActive` (`self.Thruster30`) Active false))
  (if AffectBack
    (`ActorComponent.SetActive` (`self.Thruster01`) Active false)
    (`ActorComponent.SetActive` (`self.Thruster11`) Active false)
    (`ActorComponent.SetActive` (`self.Thruster21`) Active false)
    (`ActorComponent.SetActive` (`self.Thruster31`) Active false)))

(fn `SetText`
  (params (Line0 :type Text) (Line1 :type Text) (Line2 :type Text))
  (`TextRenderComponent.K2_SetText` (`self.TRLine0`) Line0)
  (`TextRenderComponent.K2_SetText` (`self.TRLine1`) Line1)
  (`TextRenderComponent.K2_SetText` (`self.TRLine2`) Line2))

(fn `UserConstructionScript`
  (`self.SetText` (`self.Line0`) (`self.Line1`) (`self.Line2`)))