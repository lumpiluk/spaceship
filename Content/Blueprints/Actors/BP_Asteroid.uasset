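; Asteroid obstacle that moves along -X toward the player and explodes when hit by a laser or the player ship.
; Construction randomizes rotation, spin and, through independent picks, the static and destructible meshes.
; Hits notify AsteroidObserver, then swap the static mesh for the destructible with radial damage and particles; only laser hits disable collision.
; I_Moveable lets an observer set speed and destroy it after Tick reports it out of range.
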(event `self.ReceiveBeginPlay`)

(event `self.ReceiveActorBeginOverlap`
  (params (OtherActor :type "Actor Object Reference")))

(event `self.ReceiveTick`
  (params (DeltaSeconds :type "Float (single-precision)"))
  (if (< (.x (.location (`self.GetTransform`))) (`self.BehindPlayerX`))
    ;[1 1 1] Notify observer that this actor can now be destroyed
    (`/Game/Blueprints/Interfaces/I_MoveableObserver.MoveableOutOfRange` (`self.MoveableObserver`) self)))

(event `/Game/Blueprints/Interfaces/I_Moveable.SetOncomingSpeed`
  (params (NewSpeed :type "Float (single-precision)"))
  ;[1 1 1] I_Moveable implementations
  (set `MovementComponent.Velocity` (`KismetMathLibrary.MakeVector` (* NewSpeed -1.0)) (`self.ProjectileMovement`)))

(event `/Game/Blueprints/Interfaces/I_Moveable.SetObserver`
  (params (Observer :type "/Game/Blueprints/Interfaces/I_MoveableObserver Interface"))
  ;[1 1 1] I_Moveable implementations
  (set `self.MoveableObserver` Observer))

(event `/Game/Blueprints/Interfaces/I_Moveable.DestroyMoveableActor`
  ;[1 1 1] I_Moveable implementations
  (`self.K2_DestroyActor`))

(event `self.AsteroidMesh.OnComponentBeginOverlap`
  (params (OtherActor :type "Actor Object Reference") (OtherComp :type "PrimitiveComponent Object Reference") (OtherBodyIndex :type Integer) (bFromSweep :type Boolean) (SweepResult :type "HitResult Structure (by ref)"))
  (bind _asteroidmesh (`self.AsteroidMesh`))
  (bind _asteroiddestructible (`self.AsteroidDestructible`))
  (if (`self.ActorHasTag` OtherActor "LaserProjectile")
    ;[1 1 1] Notify asteroid observer of laser hit
    (`/Game/Blueprints/Interfaces/I_AsteroidObserver.AsteroidHitByLaser` (`self.AsteroidObserver`) self)
    (`PrimitiveComponent.SetCollisionEnabled` (`self.AsteroidMesh`) "NoCollision")
    ;[1 1 1] Explode asteroid
    (`SceneComponent.SetVisibility` _asteroidmesh false false :!label _label)
    (`SceneComponent.SetHiddenInGame` _asteroidmesh true false)
    (`SceneComponent.SetVisibility` _asteroiddestructible true false)
    (`DestructibleComponent.ApplyRadiusDamage` _asteroiddestructible 1.0 (`SceneComponent.K2_GetComponentLocation` _asteroiddestructible) 1000.0 20000.0 false)
    (`ActorComponent.Activate` (`self.ExplosionParticles`) false)
    (elif (`self.ActorHasTag` OtherActor "SpaceshipPlayer")
      ;[1 1 1] Notify asteroid observer of player hit
      (`/Game/Blueprints/Interfaces/I_AsteroidObserver.AsteroidHitByPlayer` (`self.AsteroidObserver`) self)
      (goto _label))))

(event `DestroyAfterSeconds`
  (params (DestructionDelay :type "Float (double-precision)"))
  (`KismetSystemLibrary.K2_SetTimerDelegate` (delegate `DestroyNow`) DestructionDelay))

(event `DestroyNow`
  (`self.K2_DestroyActor`))

(fn `Randomize`
  (bind _rotationratemax (`self.RotationRateMax`))
  (bind _returnvalue (`KismetMathLibrary.RandomIntegerInRange` 0 (- (`KismetArrayLibrary.Array_Length` (`self.AsteroidDestructibles`)) 1)))
  ;[1 1 1] Set random asteroid mesh
  (`DestructibleComponent.SetDestructibleMesh` (`self.AsteroidDestructible`) (`KismetArrayLibrary.Array_Get` (`self.AsteroidDestructibles`) _returnvalue))
  (`StaticMeshComponent.SetStaticMesh` (`self.AsteroidMesh`) (`KismetArrayLibrary.Array_Get` (`self.AsteroidMeshes`) _returnvalue))
  ;[1 1 1] Set random rotation
  (`self.SetActorRotation` (`KismetMathLibrary.RandomRotator` true))
  ;[1 1 1] Set random rotation rate
  (set `RotatingMovementComponent.RotationRate` (`KismetMathLibrary.MakeRotator` (`KismetMathLibrary.RandomFloatInRange` 0.0 _rotationratemax) (`KismetMathLibrary.RandomFloatInRange` 0.0 _rotationratemax) (`KismetMathLibrary.RandomFloatInRange` 0.0 _rotationratemax)) (`self.RotatingMovement`)))

(fn `UserConstructionScript`
  (`self.Randomize`))