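; BP_ParticlePtRing is an actor that builds a ring of points, apparently for particle placement going by its name.
; Its construction script adds eight evenly spaced arrow components on a circle in the local YZ plane, using sine and cosine for the offsets.
; Each arrow is stored in the Locations array, and the event graph has no runtime logic.
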(event `self.ReceiveBeginPlay`)

(event `self.ReceiveActorBeginOverlap`
  (params (OtherActor :type "Actor Object Reference")))

(event `self.ReceiveTick`
  (params (DeltaSeconds :type "Float (single-precision)")))

(fn `UserConstructionScript`
  (for _index (range 8)
    (bind _returnvalue (* (`KismetMathLibrary.Conv_IntToDouble` _index) (/ (`KismetMathLibrary.GetPI`) 4.0)))
    (bind _returnvalue_2 (`AddComponent|Arrow Component_1` :`RelativeTransform` (`KismetMathLibrary.MakeTransform` (`KismetMathLibrary.MakeVector` 0.0 (* 100.0 (`KismetMathLibrary.Cos` _returnvalue)) (* 100.0 (`KismetMathLibrary.Sin` _returnvalue))))))
    (`KismetArrayLibrary.Array_Add` (`self.Locations`) _returnvalue_2)))