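; BP_Util is a utility Blueprint that maintains a leaderboard of space-game scores, ranked by lowest time.
; HighscoresInsert linearly scans the list to place a new score before the first slower one, or appends it if none is found.
; It then removes entries from the end to keep the list within the given capacity.
; TestHighscoresInsert exercises this with a sample score and prints the resulting list on screen.
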(fn HighscoresInsert
  (params (Highscores :type Array%20of%20T%20Space%20Game%20Score%20Structures) (Capacity :type Integer) (NewScore :type T%20Space%20Game%20Score%20Structure))
  (bind _returnvalue (Utilities|Array|Length Highscores))
  (bind _returnvalue_2 (- _returnvalue Capacity))
  (bind _returnvalue_3 (Math|Integer|Clamp(Integer) _returnvalue_2 0 100))
  (if (> (Utilities|Array|Length Highscores) 0)
    ;[1 1 1] Insert into correct position (runs in O(n), n = length of Highscores)
    (bind (_array_element _array_index) (Utilities|Array|ForEachLoopwithBreak Highscores :!label _label)
      (:LoopBody
        (if (< (.Time (Utilities|Struct|BreakT_SpaceGameScore NewScore)) (.Time (Utilities|Struct|BreakT_SpaceGameScore _array_element)))
          (Utilities|Array|Insert Highscores NewScore (Math|Integer|Clamp(Integer) _array_index 0 (- (Utilities|Array|Length Highscores) 1)))
          (LocalVariables|SetInserted true)
          (goto _label Break)))
      (:Completed
        (if (LocalVariables|GetInserted)
          _
          (else
            (Utilities|Array|Add Highscores NewScore :!label _label_2)))
        ;[1 1 1] Remove excess items
        (if (!= _returnvalue_3 0)
          (for _index (range 1 _returnvalue_3)
            (Utilities|Array|RemoveIndex Highscores (- (Utilities|Array|Length Highscores) 1))))
        (return)))
    (else
      (goto _label_2))))

(fn TestHighscoresInsert
  (bind _scores (LocalVariables|GetScores))
  (CallFunction|HighscoresInsert _scores 10 (Utilities|Struct|MakeT_SpaceGameScore "NewPlayer" 5.0))
  (Development|PrintString 0 "Test Scores:" true true "(R=0.000000,G=0.660000,B=1.000000,A=1.000000)" 1e+01)
  (for _array_element _scores
    (Development|PrintText 0 (Utilities|Text|FormatText "{Name}: {Time}" (Utilities|Text|ToText(String) (.PlayerName (Utilities|Struct|BreakT_SpaceGameScore _array_element))) (Utilities|Text|ToText(Float) (.Time (Utilities|Struct|BreakT_SpaceGameScore _array_element)) "HalfToEven" true 1 324 1)) true true "(R=0.000000,G=0.660000,B=1.000000,A=1.000000)" 1e+01)))